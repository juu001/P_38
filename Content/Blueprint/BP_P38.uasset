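; BP_P38 is a player-controlled aircraft that flies forward continuously at a constant speed.
; It enables input from player controller 0 on BeginPlay, then maps the Pitch and Roll axes to local rotation scaled by RotationSpeed and delta time.
; Tick spins the Right and Left components in opposite roll directions and moves the actor along its local forward axis, so steering comes purely from orientation.
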(event `InputAxis|Pitch`
  (params (AxisValue :type "Float (single-precision)"))
  (`self.K2_AddActorLocalRotation` (`KismetMathLibrary.MakeRotator` 0.0 (* AxisValue (`GameplayStatics.GetWorldDeltaSeconds`) (`self.RotationSpeed`)))))

(event `self.ReceiveBeginPlay`
  (`self.EnableInput` (`GameplayStatics.GetPlayerController` 0)))

(event `InputAxis|Roll`
  (params (AxisValue :type "Float (single-precision)"))
  (`self.K2_AddActorLocalRotation` (`KismetMathLibrary.MakeRotator` (* (`self.RotationSpeed`) (`GameplayStatics.GetWorldDeltaSeconds`) AxisValue))))

(event `self.ReceiveTick`
  (params (DeltaSeconds :type "Float (single-precision)"))
  ;[1 1 1] right
  (`SceneComponent.K2_AddLocalRotation` (`self.Right`) (`KismetMathLibrary.MakeRotator` (* (`GameplayStatics.GetWorldDeltaSeconds`) 1000.0)) false false)
  ;[1 1 1] left
  (`SceneComponent.K2_AddLocalRotation` (`self.Left`) (`KismetMathLibrary.MakeRotator` (* -1 (* (`GameplayStatics.GetWorldDeltaSeconds`) 1000.0))) false false)
  ;[1 1 1] goahead
  (`self.K2_AddActorLocalOffset` (`KismetMathLibrary.MakeVector` (* 100 (`GameplayStatics.GetWorldDeltaSeconds`)))))

(fn `UserConstructionScript`)